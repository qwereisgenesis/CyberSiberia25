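; Level boundary actor that warns the player with a danger widget when BP_PlayerCharacter leaves its Sphere.
; End overlap adds a new W_danger1 to the viewport.
; Begin overlap clears the warning by removing all widgets, then recreates the HUD, help, energy, speed and score widgets.
; Widget references are not stored, so each crossing creates fresh instances.
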(event `self.Sphere.OnComponentEndOverlap`
  (params (OverlappedComponent :type "PrimitiveComponent Object Reference") (OtherActor :type "Actor Object Reference") (OtherComp :type "PrimitiveComponent Object Reference") (OtherBodyIndex :type Integer))
  (cast `/Game/ThirdPerson/Blueprints/BP_PlayerCharacter` OtherActor)
  (bind _returnvalue (`|CreateWidget` "/Game/POTAPOV/w_danger1.w_danger1_C"))
  (`UserWidget.AddToViewport` _returnvalue 0))

(event `self.Sphere.OnComponentBeginOverlap`
  (params (OverlappedComponent :type "PrimitiveComponent Object Reference") (OtherActor :type "Actor Object Reference") (OtherComp :type "PrimitiveComponent Object Reference") (OtherBodyIndex :type Integer) (bFromSweep :type Boolean) (SweepResult :type "HitResult Structure (by ref)"))
  (cast `/Game/ThirdPerson/Blueprints/BP_PlayerCharacter` OtherActor)
  (`WidgetLayoutLibrary.RemoveAllWidgets`)
  (`|ExecutionSequence`
    (:`then_0`
      ;[0.5204 1 0.2807] Add Widgets
      (bind _returnvalue (`|CreateWidget` "/Game/ThirdPerson/Blueprints/W_HUD.W_HUD_C"))
      (`UserWidget.AddToViewport` _returnvalue 0))
    (:`then_1`
      (bind _returnvalue_2 (`|CreateWidget` "/Game/ThirdPerson/Blueprints/W_help.W_help_C"))
      (`UserWidget.AddToViewport` _returnvalue_2 0))
    (:`then_2`
      (bind _returnvalue_3 (`|CreateWidget` "/Game/POTAPOV/w_energy.w_energy_C"))
      (`UserWidget.AddToViewport` _returnvalue_3 0))
    (:`then_3`
      (bind _returnvalue_4 (`|CreateWidget` "/Game/POTAPOV/w_Speed.w_Speed_C"))
      (`UserWidget.AddToViewport` _returnvalue_4 0))
    (:`then_4`
      (bind _returnvalue_5 (`|CreateWidget` "/Game/POTAPOV/W_score.W_score_C"))
      (`UserWidget.AddToViewport` _returnvalue_5 0))))

(fn `UserConstructionScript`)