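; bp_ring is a one-time score pickup collected by the player character.
; BeginPlay caches a reference to BP_ThirdPersonGameMode.
; When BP_PlayerCharacter overlaps the Sphere, a DoOnce gate adds ADDSCORE to the game mode's Score and spawns an explosion particle at the Cube component.
; The actor destroys itself after a short delay.
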(event `self.ReceiveBeginPlay`
  (bind _asbp_third_person_game_mode (cast `/Game/ThirdPerson/Blueprints/BP_ThirdPersonGameMode` (`GameplayStatics.GetGameMode`)))
  (set `self.As BP Third Person Game Mode` _asbp_third_person_game_mode))

(event `self.Sphere.OnComponentBeginOverlap`
  (params (OverlappedComponent :type "PrimitiveComponent Object Reference") (OtherActor :type "Actor Object Reference") (OtherComp :type "PrimitiveComponent Object Reference") (OtherBodyIndex :type Integer) (bFromSweep :type Boolean) (SweepResult :type "HitResult Structure (by ref)"))
  (bind _as_bp_third_person_game_mode (`self.As BP Third Person Game Mode`))
  (cast `/Game/ThirdPerson/Blueprints/BP_PlayerCharacter` OtherActor)
  (`/Engine/EditorBlueprintResources/StandardMacros.DoOnce` false
    (:`Completed`
      (set `/Game/ThirdPerson/Blueprints/BP_ThirdPersonGameMode.score` (+ (`self.ADD SCORE`) (`/Game/ThirdPerson/Blueprints/BP_ThirdPersonGameMode.score` _as_bp_third_person_game_mode)) _as_bp_third_person_game_mode)
      (`GameplayStatics.SpawnEmitterAtLocation` "/Game/StarterContent/Particles/P_Explosion.P_Explosion" (`SceneComponent.K2_GetComponentLocation` (`self.Cube`)) (struct) (2.0 2.0 2.0))
      (`KismetSystemLibrary.Delay` 0.5)
      (`self.K2_DestroyActor`))))

(fn `UserConstructionScript`)